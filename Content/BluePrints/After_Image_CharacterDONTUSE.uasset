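; After-image Paper2D character, marked DONTUSE by name, that can move and jump on its own input bindings.
; Enhanced Input drives horizontal movement, control-rotation facing and jumping, while a custom event also triggers jumps.
; Jumping or walking off a ledge sends the animation instance to its Airborne jump node.
; BeginPlay caches BP_Player, but the logic copying its location, velocity and rotation is disconnected.
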(event `self.ReceiveBeginPlay`
  ; Sets a Reference for the Player when spawned
  (bind _asbp_player (cast `/Game/BluePrints/Player/BP_Player` (`GameplayStatics.GetPlayerCharacter` 0)))
  (set `self.As BP Player` _asbp_player)
  (`PaperFlipbookComponent.SetFlipbook` (`self.Sprite`) null))

(event `After_Image_Jump`
  (`self.Jump`))

(event `EnhancedInput|/Game/Input/Actions/IA_Jump`
  (params (ActionValue :type Boolean) (ElapsedSeconds :type "Float (double-precision)") (TriggeredSeconds :type "Float (double-precision)") (InputAction :type "InputAction Object Reference" :default "/Game/Input/Actions/IA_Jump.IA_Jump"))
  ; Jumping
  (:`Started`
    (`self.Jump`))
  (:`Completed`
    (`self.StopJumping`)))

(event `self.OnWalkingOffLedge`
  (params (PreviousFloorImpactNormal :type "Vector Structure (by ref)") (PreviousFloorContactNormal :type "Vector Structure (by ref)") (PreviousLocation :type "Vector Structure (by ref)") (TimeDelta :type "Float (single-precision)"))
  ; Jumping
  (`PaperZDAnimInstance.JumpToNode` (`PaperZDAnimationComponent.AnimInstance` (`self.AnimationComponent`)) "Airborne" "None" :!label _label))

(event `self.OnJumped`
  ; Jumping
  (goto _label))

(event `EnhancedInput|/Game/Input/Actions/IA_Move`
  (params (ActionValue :type "Float (double-precision)") (ElapsedSeconds :type "Float (double-precision)") (TriggeredSeconds :type "Float (double-precision)") (InputAction :type "InputAction Object Reference" :default "/Game/Input/Actions/IA_Move.IA_Move"))
  (bind _returnvalue (`self.GetController`))
  (:`Triggered`
    (`self.AddMovementInput` (1.0 0.0 0.0) ActionValue)
    (`/Engine/EditorBlueprintResources/StandardMacros.IsValid` _returnvalue
      (:`Is Valid`
        (`Controller.SetControlRotation` _returnvalue (select `bool` (> ActionValue 0.0) :`false` (`KismetMathLibrary.MakeRotator` 0.0 0.0 180.0) :`true` (`KismetMathLibrary.MakeRotator` 0.0)))))))

(fn `UserConstructionScript`)