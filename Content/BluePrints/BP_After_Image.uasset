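; Player after-image ghost that trails BP_Player using the oldest transform stored in the player's position tracker component.
; Each Tick it sets its flipbook (respawn or after-image), moves via VInterpTo with that transform as Current, copies its rotation, then resolves velocity.
; It raises its CustomTimeDilation while the player's TimeSlow is active, and prints that value every frame as debug output.
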(event `self.ReceiveBeginPlay`
  (bind _asbp_player (cast `/Game/BluePrints/Player/BP_Player` (`GameplayStatics.GetPlayerCharacter` 0)))
  (set `self.As BP Player` _asbp_player)
  (`PaperFlipbookComponent.SetFlipbook` (`self.Sprite`) "/Game/BluePrints/Player/Assests/Flipbooks/FB_Player_Idle.FB_Player_Idle"))

(event `self.ReceiveTick`
  (params (DeltaSeconds :type "Float (single-precision)"))
  (`self.Update_Animation`)
  (`self.After_Image_Movement` DeltaSeconds)
  (`self.Resolve_Movement`)
  (`KismetSystemLibrary.PrintString` (`KismetStringLibrary.Conv_DoubleToString` (`self.CustomTimeDilation`))))

(event `Update_Animation`
  (if (`self.Respawning?`)
    (`PaperFlipbookComponent.SetFlipbook` (`self.Sprite`) "/Game/BluePrints/Player/Assests/Flipbooks/FB_Player_Respawn.FB_Player_Respawn")
    (else
      (`PaperFlipbookComponent.SetFlipbook` (`self.Sprite`) "/Game/Assests/After_Images/Flipbook/After_Image.After_Image"))))

(fn `Add_velocity`
  (params (Direction :type "Vector Structure") (Scale :type "Float (double-precision)"))
  (set `self.Added_Velocity` (+ (* Direction (* Scale (`GameplayStatics.GetWorldDeltaSeconds`))) (`self.Added_Velocity`))))

(fn `After_Image_Movement`
  (params (DeltaTime :type "Float (single-precision)"))
  (bind (_transform_location _transform_rotation) (`KismetMathLibrary.BreakTransform` (`/Game/BluePrints/BPC_Position_Tracker.Get_Oldest_Transform` (`/Game/BluePrints/Player/BP_Player.BPC_Position_Tracker` (`self.As BP Player`)))))
  (bind _transform_location_2 (`KismetMathLibrary.BreakTransform` (`/Game/BluePrints/BPC_Position_Tracker.Get_Oldest_Transform` (`/Game/BluePrints/Player/BP_Player.BPC_Position_Tracker` (`self.As BP Player`)))))
  (bind _transform_location_3 (`KismetMathLibrary.BreakTransform` (`/Game/BluePrints/BPC_Position_Tracker.Get_Oldest_Transform` (`/Game/BluePrints/Player/BP_Player.BPC_Position_Tracker` (`self.As BP Player`)))))
  (if (`/Game/BluePrints/Player/BP_Player.Time_Slow` (`self.As BP Player`))
    (set `self.CustomTimeDilation` 5.0)
    (else
      (set `self.CustomTimeDilation` 1.0)))
  ; Confirm if player is valid
  (bind _as_bp_player (`self.As BP Player`)
    (:`then`
      (if (`/Game/BluePrints/BPC_Position_Tracker.is_Tracking?` (`/Game/BluePrints/Player/BP_Player.BPC_Position_Tracker` _as_bp_player))
        (`self.K2_SetActorLocation` (`KismetMathLibrary.VInterpTo` _transform_location_2 (`self.K2_GetActorLocation`) DeltaTime 3.0))
        ; Setting the Direction for the Ghost
        (set `self.Direction` (- _transform_location_3 (`self.K2_GetActorLocation`)))
        (`self.K2_SetActorRotation` _transform_rotation)))
    (:`else`)))

(fn `After_Image_Ref`
  (returns (After_Image_REF :type "/Game/BluePrints/BP_After_Image Object Reference"))
  (return self))

(fn `Resolve_Movement`
  (locals (Location_Before :type "Vector Structure"))
  (set `local.Location_Before` (`self.K2_GetActorLocation`))
  (`|ExecutionSequence`
    (:`then_0`
      (`self.K2_SetActorLocation` (+ (`self.K2_GetActorLocation`) (* (+ (`self.Velocity`) (`self.Added_Velocity`)) (`GameplayStatics.GetWorldDeltaSeconds`)))))
    (:`then_1`
      (set `self.Velocity` (/ (- (`self.K2_GetActorLocation`) (`local.Location_Before`)) (`GameplayStatics.GetWorldDeltaSeconds`)))
      (set `self.Added_Velocity` (0.0 0.0 0.0)))))

(fn `UserConstructionScript`)