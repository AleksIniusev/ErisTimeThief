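; Actor component that records its owner's recent transforms and spawns a BP_After_Image ghost at the oldest one.
; Activation prefills a fixed-size buffer sized by TimeToTrack over Interval, then a looping timer rolls it forward, offsetting Y to keep the ghost behind the player.
; Tracking starts deactivated; deactivation clears the timer and destroys the ghost.
; Helper functions expose the oldest transform and evenly spaced history samples.
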(event `self.ReceiveBeginPlay`
  (`self.Deactiviate_Tracking`))

(event `Activiate_Tracking`
  ; Activiates/Deactiviates Tracking
  (set `self.is_Tracking?` true)
  ;;[0.4588 0.4588 0.4588 0.502] Gets the Position Data of the Player/Owner
  (`self.Initialize_Position_Data`)
  ;;[0.4588 0.4588 0.4588 0.502] Updates the current position and new position in the interval
  (bind _returnvalue (`KismetSystemLibrary.K2_SetTimerDelegate` (`|CreateDelegate` :!event `Update_Position_Data`) (`self.Interval`) true))
  (set `self.Update_Data_Handle` _returnvalue)
  (`self.Spawns_After_Image`)
  (`KismetSystemLibrary.Delay` 1.0)
  (set `/Game/BluePrints/BP_After_Image.Respawning?` false (`self.Ghost_Ref`)))

(event `self.ReceiveTick`
  (params (DeltaSeconds :type "Float (single-precision)")))

(event `Deactiviate_Tracking`
  ; Activiates/Deactiviates Tracking
  (set `self.is_Tracking?` false)
  ;;[0.4588 0.4588 0.4588 0.502] Invalidates the event timer of Update_Position_Data
  (`KismetSystemLibrary.K2_ClearAndInvalidateTimerHandle` (`self.Update_Data_Handle`))
  (bind _ghost_ref (`self.Ghost_Ref`)
    (:`then`
      (`Actor.K2_DestroyActor` _ghost_ref))
    (:`else`)))

(fn `Get_Oldest_Transform`
  (returns (Transform :type "Transform Structure"))
  (return (`|GetArrayItem` (`self.Position_Data`))))

(fn `Initialize_Position_Data`
  (locals (Array_Size :type Integer :default 0))
  (bind (_returnvalue_location _returnvalue_rotation _returnvalue_scale) (`KismetMathLibrary.BreakTransform` (`Actor.GetTransform` (`self.GetOwner`))))
  (bind _output_get (set `local.Array_Size` (`KismetMathLibrary.Round` (/ (`self.Time_To_Track`) (`self.Interval`)))))
  (for _index (range _output_get)
    ; Inserts the Players/Owner Transform into the array
    (`KismetArrayLibrary.Array_Insert` (`self.Position_Data`) (`KismetMathLibrary.MakeTransform` (- _returnvalue_location (0.0 1.0 0.0)) _returnvalue_rotation _returnvalue_scale) _index))
  ; Ensures the size of array = the array size variable to fit the algrothim of the array size
  (`KismetArrayLibrary.Array_Resize` (`self.Position_Data`) (`local.Array_Size`)))

(fn `Sample_Position_Data`
  (params (Sample_Count :type Integer))
  (returns (Sample_Transform :type "Array of Transform Structure"))
  (locals (Sample_Gap :type Integer :default 7) (Sampled_Transforms :type "Array of Transform Structure") (Index :type Integer))
  (set `local.Sample_Gap` (/ (`KismetArrayLibrary.Array_Length` (`self.Position_Data`)) Sample_Count))
  (while (< (`local.Index`) (`KismetArrayLibrary.Array_Length` (`self.Position_Data`)))
    (`KismetArrayLibrary.Array_Add` (`local.Sampled_Transforms`) (`|GetArrayItem` (`self.Position_Data`) (`local.Index`)))
    (set `local.Index` (+ (`local.Index`) (`local.Sample_Gap`))))
  (return (`local.Sampled_Transforms`)))

(fn `Spawns_After_Image`
  (bind (_transform_location _transform_rotation _transform_scale) (`KismetMathLibrary.BreakTransform` (`self.Get_Oldest_Transform`)))
  ; Check if it already exists if so Destroy
  (bind _ghost_ref (`self.Ghost_Ref`)
    (:`then`
      (`Actor.K2_DestroyActor` _ghost_ref))
    (:`else`
      _))
  ; Spawns the after Image from the Oldest Position of the Player/Owner
  (bind _returnvalue (`|SpawnActorFromClass` "/Game/BluePrints/BP_After_Image.BP_After_Image_C" (`KismetMathLibrary.MakeTransform` (- _transform_location (0.0 0.1 20.0)) _transform_rotation _transform_scale) "Undefined" "MultiplyWithRoot" null null))
  (set `self.Ghost_Ref` _returnvalue)
  (set `/Game/BluePrints/BP_After_Image.Respawning?` true (`self.Ghost_Ref`)))

(fn `Update_Position_Data`
  (bind _position_data (`self.Position_Data`))
  (bind (_returnvalue_location _returnvalue_rotation _returnvalue_scale) (`KismetMathLibrary.BreakTransform` (`Actor.GetTransform` (`self.GetOwner`))))
  (bind _output_location (`KismetMathLibrary.BreakTransform` (`|GetArrayItem` _position_data)))
  ; Removes the First Position
  (`KismetArrayLibrary.Array_Remove` _position_data)
  ; Where ever the player/owner is in the world the data gets added
  (`KismetArrayLibrary.Array_Add` _position_data (`KismetMathLibrary.MakeTransform` (- _returnvalue_location (0.0 1.0 0.0)) _returnvalue_rotation _returnvalue_scale))
  ;[0.1058 0.01667 0.15 0.5] TESTING!!!!!
  (if (`self.Show_Debug_Sphere`)
    (`KismetSystemLibrary.DrawDebugSphere` _output_location 100.0 12 (struct :`R` 1.0 :`G` 1.0 :`B` 1.0 :`A` 1.0) (`self.Interval`))))